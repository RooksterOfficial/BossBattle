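; Player controller for BossBattle's top-down, click-to-move hero play on a client-server setup.
; On spawn it shows the in-game UI, then the server records the hero pick, spawns that hero at a random PlayerStart and possesses it with a separate AI controller.
; Left clicks send the cursor hit to that controller's MoveToLocation and drop an indicator, while Tick eases the player's camera pawn after the hero.
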(event Custom|Server_Spawn_Player
  (params (NewHeroID :type E_HeroID%20Enum :default "NewEnumerator0"))
  ;[1 0.5911 0] Server: Spawn our Topdown AI Character
  (bind _asboss_battle_game_state (Utilities|Casting|CastToBossBattle_GameState (Game|GetGameState)))
  (Default|UpdateSelectedHeroes _asboss_battle_game_state NewHeroID "NewEnumerator2")
  ;;[1 1 1] Selects a random player start for the AI Character to Spawn in
  (bind _outactors (Actor|GetAllActorsOfClass "/Script/Engine.PlayerStart"))
  (Utilities|FlowControl|DoOnce false
    (:Completed
      (bind _newparam (CallFunction|GetHeroReftoSpawn NewHeroID))
      (bind _returnvalue (Game|SpawnActorfromClass _newparam (Math|Conversions|ToTransform(Vector) (Transformation|GetActorLocation (Utilities|Array|Get(acopy) _outactors (Math|Random|RandomIntegerinRange 0 (Utilities|Array|LastIndex _outactors))))) "Undefined" 0 0))
      (bind _asserver_ai_character (Utilities|Casting|CastToServer_AI_Character _returnvalue))
      (Variables|Default|SetServer_AI_Character _asserver_ai_character)
      (bind _returnvalue_2 (Game|SpawnActorfromClass "/Game/BossBattle/Blueprints/Unit/Server_AI_Controller.Server_AI_Controller_C" (Math|Conversions|ToTransform(Vector) (Transformation|GetActorLocation (Utilities|Array|Get(acopy) _outactors (Math|Random|RandomIntegerinRange 0 (Utilities|Array|LastIndex _outactors))))) "Undefined" 0 0))
      (Variables|Default|SetServer_AI_Controller _returnvalue_2)
      (Pawn|Possess (Variables|Default|GetServer_AI_Controller) (Variables|Default|GetServer_AI_Character))
      (Transformation|SetActorLocation (Pawn|GetControlledPawn) (Transformation|GetActorLocation (Variables|Default|GetServer_AI_Character)) false true))))

(event Custom|Server_Move_Server_Character
  (params (Destination :type Vector))
  (bind _server_ai_controller (Variables|Default|GetServer_AI_Controller))
  ;[1 0.5911 0] Server: Move AI Character to controlling clients mouse position
  (Utilities|IsValid _server_ai_controller
    (:Is%20Valid
      (AI|Navigation|MovetoLocation _server_ai_controller Destination -1.0 true true false true 0))))

(event Custom|SpawnHero
  (params (HeroID :type E_HeroID%20Enum :default "NewEnumerator0"))
  ;[1 1 1] Spawn our AI Character on the server
  (CallFunction|ServerSpawnPlayer HeroID)
  ;[1 1 1] Show our mouse cursor
  (Variables|Default|SetbShowMouseCursor true)
  ;[1 1 1] Adds ingame UI to Viewport
  (bind _returnvalue (UserInterface|CreateWidget "/Game/BossBattle/UI/Ingame_WB.Ingame_WB_C" (Game|GetPlayerController 0)))
  (UserInterface|Viewport|AddtoViewport _returnvalue 0)
  (Variables|Default|SetbInputEnabled true))

(event EventTick
  (params (DeltaSeconds :type Float%20%28single-precision%29))
  ;[1 1 1] Client: Sets clients pawn location every tick (Our camera in game)
  (Utilities|IsValid (Variables|Default|GetServer_AI_Character)
    (:Is%20Valid
      (Transformation|SetActorLocation (Pawn|GetControlledPawn) (Math|Interpolation|VInterpTo (Transformation|GetActorLocation (Pawn|GetControlledPawn)) (Transformation|GetActorLocation (Variables|Default|GetServer_AI_Character)) DeltaSeconds 1e+01) false false))))

(event Input|MouseEvents|LeftMouseButton
  (params (Key :type Key%20Structure :default "None"))
  (bind _hitresult (Game|Player|GetHitResultUnderCursorbyChannel "TraceTypeQuery1" true))
  (bind (_bblockinghit _binitialoverlap _time _distance _location) (Collision|BreakHitResult _hitresult))
  ;[1 1 1] Client: Move Server AI Character
  (:Pressed
    (if (Variables|Default|GetbInputEnabled)
      (if _bblockinghit
        (CallFunction|ServerMoveServerCharacter _location)
        ;;[1 1 1] Spawn MoveToLocation_Indicator actor
        (Game|SpawnActorfromClass "/Game/BossBattle/Blueprints/Player/MoveToLocation_Indicator.MoveToLocation_Indicator_C" (Math|Conversions|ToTransform(Vector) _location) "Undefined" 0 0)))))

(fn ConstructionScript)

(fn GetHeroReftoSpawn
  (params (HeroID :type E_HeroID%20Enum :default "NewEnumerator0"))
  (switch Utilities|FlowControl|Switch|SwitchonE_HeroID HeroID
    (:NewEnumerator0
      (return "/Game/BossBattle/Blueprints/Unit/Heroes/Rippers/BP_PhantomRipper.BP_PhantomRipper_C"))
    (:NewEnumerator1
      (return "/Game/BossBattle/Blueprints/Unit/Heroes/Healers/BP_UndeadButler.BP_UndeadButler_C"))))