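; BaseUnit is a combat unit base Blueprint that auto-attacks a target, takes damage and dies.
; AutoAttack replays a montage while a living target overlaps AttackRadius, otherwise retries on a timer; its "Attack" notify triggers damage and sound.
; RecieveDamage lowers health, spawns a floating damage number and starts death, whose montage notify freezes the mesh.
; BeginPlay spawns a UnitClassType actor, construction offsets the attack sphere, and an XP-scaling loop is unconnected.
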(event Custom|AutoAttack
  ;[1 1 1] AutoAttack
  (bind _target (Variables|Default|GetTarget)
    (:then
      (if (and (> (Variables|BaseUnit_C|GetHealth_Current _target) 0.0) (Collision|IsOverlappingActor (Variables|Default|GetAttackRadius) _target :!class /Script/Engine.PrimitiveComponent))
        (bind _notifyname (Animation|Montage|PlayMontage (Variables|Character|GetMesh) (Variables|Default|GetAttackMontage))
          (:OnCompleted
            (CallFunction|AutoAttack))
          (:OnNotifyBegin
            (if (Utilities|Name|Equal(Name) _notifyname "Attack")
              (Utilities|FlowControl|Sequence
                (:then_0
                  (CallFunction|SendDamage))
                (:then_1
                  (Audio|PlaySoundatLocation (Variables|Default|GetAttackSfx) (Transformation|GetActorLocation) "0, 0, 0" 1.0 1.0 0.0 0 0 0))))))
        (else
          (Utilities|Time|SetTimerbyEvent (delegate Custom|AutoAttack) 0.5))))
    (:else)))

(event Custom|InitiateDeath
  ;[1 1 1] Death
  (if (not (Animation|Montage|MontageIsPlaying (Components|SkeletalMesh|GetAnimInstance (Variables|Character|GetMesh)) (Variables|Default|GetDeathMontage)))
    (Utilities|FlowControl|Sequence
      (:then_0
        (Audio|PlaySoundatLocation (Variables|Default|GetDeathSfx) (Transformation|GetActorLocation) "0, 0, 0" 1.0 1.0 0.0 0 0 0))
      (:then_1
        (bind _notifyname (Animation|Montage|PlayMontage (Variables|Character|GetMesh) (Variables|Default|GetDeathMontage))
          (:OnNotifyBegin
            (if (Utilities|Name|Equal(Name) _notifyname "EndSequence")
              (Components|Timeline|SetPlayRate (Variables|Character|GetMesh) 0.0))))))))

(event EventBeginPlay
  (Game|SpawnActorfromClass (Variables|Default|GetUnitClassType) (Math|Transform|MakeTransform "0, 0, 0" "0, 0, 0" "1,1,1") "AlwaysSpawn" self 0))

(event Collision|EventActorBeginOverlap
  (params (OtherActor :type Actor%20Object%20Reference)))

(event EventTick
  (params (DeltaSeconds :type Float%20%28single-precision%29)))

(fn ConstructionScript
  (bind _attackradius (Variables|Default|GetAttackRadius))
  (Utilities|FlowControl|Sequence
    (:then_0
      (Transformation|SetRelativeLocation _attackradius (Math|Vector|MakeVector (* (Variables|/Script/Engine.SphereComponent|GetSphereRadius _attackradius) 0.5) 0.0 0.0) false false))
    (:then_1)))

(fn SendDamage
  (CallFunction|RecieveDamage (Variables|Default|GetTarget) (Variables|Default|GetAttackDamage)))

(fn RecieveDamage
  (params (DamageRecieved :type Float%20%28single-precision%29))
  (Utilities|FlowControl|Sequence
    (:then_0
      ;[1 1 1] Calculate damage taken
      (Variables|Default|SetHealth_Current (- (Variables|Default|GetHealth_Current) DamageRecieved))
      ;[1 1 1] GENERATE FLOATING DAMAGE NUMBER
      (bind _returnvalue (UserInterface|CreateWidget "/Game/Blueprints/Widget/DmgNumber.DmgNumber_C" 0 (Math|Float|Truncate DamageRecieved) (.ScreenPosition (Class|GameplayStatics|ProjectWorldtoScreen (Game|GetPlayerController 0) (Transformation|GetActorLocation) false))))
      (UserInterface|Viewport|AddtoViewport _returnvalue 0))
    (:then_1
      ;[1 1 1] TRIGGER DEATH
      (if (<= (Variables|Default|GetHealth_Current) 0.0)
        (CallFunction|InitiateDeath)))))